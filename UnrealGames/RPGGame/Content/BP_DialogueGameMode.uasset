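; Dialogue game mode that starts a conversation on BeginPlay, creating a rich dialogue widget and showing the mouse cursor.
; AdvanceDialogue builds TestTable row names from the line index, or index.reply.subindex inside a branch, then has the widget speak or show replies.
; A chosen reply enters its branch, and a missing row returns to the next main line.
; An End row calls EndConvo, which is still empty.
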(event `self.ReceiveBeginPlay`
  (`self.OnInteraction`)
  (set `PlayerController.bShowMouseCursor` true (`GameplayStatics.GetPlayerController` 0)))

(event `self.OnInteraction`
  (set `self.Index` 0)
  (bind _returnvalue (`|CreateWidget` "/Game/BluePrints/DialogueSystem/DialogueWidget_Rich.DialogueWidget_Rich_C"))
  (bind _output_get (set `self.DialogueWidget` _returnvalue))
  (add `/Game/BluePrints/DialogueSystem/DialogueWidget_Rich.OnReplyFinished` _output_get (delegate `EnterReply`))
  (`UserWidget.AddToViewport` _output_get 0)
  (`self.AdvanceDialogue`))

(event `EnterReply`
  (params (ReplyIndex :type Integer))
  (if (not (== (`self.ReplyValue`) 0))
    (`/Engine/EditorBlueprintResources/StandardMacros.IncrementInt` (`self.Index`)
      (:`  `
        _)))
  (set `self.ReplyValue` (+ ReplyIndex 1))
  (set `self.SubIndex` 0)
  (`/Game/BluePrints/DialogueSystem/DialogueWidget_Rich.SetDialogueState` (`self.DialogueWidget`) "NewEnumerator0")
  (`self.AdvanceDialogue`)
  (`KismetSystemLibrary.PrintString` "REPLYING"))

(event `AdvanceDialogue`
  (if (`|EnumEquality` (`/Game/BluePrints/DialogueSystem/DialogueWidget_Rich.DialogueState` (`self.DialogueWidget`)) "NewEnumerator0")
    (bind _output_get (set `self.TableString` (`KismetStringLibrary.Conv_IntToString` (`self.Index`))))
    (if (== (`self.ReplyValue`) 0)
      (`/Engine/EditorBlueprintResources/StandardMacros.IncrementInt` (`self.Index`)
        (:`  `
          _))
      (else
        (set `self.TableString` (`KismetStringLibrary.Concat_StrStr` _output_get "." (`KismetStringLibrary.Conv_IntToString` (`self.ReplyValue`)) "." (`KismetStringLibrary.Conv_IntToString` (`self.SubIndex`))))
        (`/Engine/EditorBlueprintResources/StandardMacros.IncrementInt` (`self.SubIndex`)
          (:`  `
            _))))
    (`KismetSystemLibrary.PrintString` (`self.TableString`) true true (struct :`R` 1.0 :`B` 0.983937 :`A` 1.0) 10.0)
    (bind _returnvalue (`|GetDataTableRow` (`self.TestTable`) (`KismetStringLibrary.Conv_StringToName` (`self.TableString`)))
      (:`then`
        (bind (_speakername _speakertext _animtype _screenside _replyarray) (break `DialogueStruct` _returnvalue))
        (switch `name` _speakername
          (:`Default`
            (`/Game/BluePrints/DialogueSystem/DialogueWidget_Rich.BeginSpeaking` (`self.DialogueWidget`) _speakername _speakertext _animtype _screenside))
          (:`Reply`
            (`/Game/BluePrints/DialogueSystem/DialogueWidget_Rich.Reply` (`self.DialogueWidget`) _replyarray)
            (`KismetSystemLibrary.PrintString` "ENTERING REPLY STATE" true true (struct :`R` 1.0 :`G` 0.827957 :`A` 1.0) 5.0))
          (:`End`
            (`self.EndConvo`))))
      (:`RowNotFound`
        (`KismetSystemLibrary.PrintString` "FAILED TO FIND ROW, aENDING CONVO" true true (struct :`R` 1.0 :`B` 0.095971 :`A` 1.0))
        (set `self.ReplyValue` 0)
        (set `self.SubIndex` 0)
        (`/Engine/EditorBlueprintResources/StandardMacros.IncrementInt` (`self.Index`)
          (:`  `
            (`self.AdvanceDialogue`)))))))

(event `EndConvo`)

(fn `UserConstructionScript`)