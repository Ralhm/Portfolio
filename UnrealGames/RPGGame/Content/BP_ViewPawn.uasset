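; BP_ViewPawn is a view pawn that keeps nearby RPG characters from cluttering the view and shows the mouse cursor on BeginPlay.
; When a living RPGCharacter enters its Sphere, it is hidden unless it is the CurrentLookCharacter.
; Leaving the Sphere makes a living character visible again, while dead characters are left untouched by both overlap events.
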(event `self.ReceiveBeginPlay`
  (set `PlayerController.bShowMouseCursor` true (`GameplayStatics.GetPlayerController` 0)))

(event `self.Sphere.OnComponentBeginOverlap`
  (params (OverlappedComponent :type "PrimitiveComponent Object Reference") (OtherActor :type "Actor Object Reference") (OtherComp :type "PrimitiveComponent Object Reference") (OtherBodyIndex :type Integer) (bFromSweep :type Boolean) (SweepResult :type "HitResult Structure (by ref)"))
  ;[1 1 1] Hide Character if get too close
  (bind _asrpgcharacter (cast `RPGCharacter` OtherActor))
  (bind _returnvalue (`RPGCharacter.IsDead` _asrpgcharacter))
  (if (not _returnvalue)
    (`self.SetActorHiddenInGame` _asrpgcharacter (not (== (`self.CurrentLookCharacter`) _asrpgcharacter)))))

(event `self.Sphere.OnComponentEndOverlap`
  (params (OverlappedComponent :type "PrimitiveComponent Object Reference") (OtherActor :type "Actor Object Reference") (OtherComp :type "PrimitiveComponent Object Reference") (OtherBodyIndex :type Integer))
  ;[1 1 1] Hide Character if get too close
  (bind _asrpgcharacter (cast `RPGCharacter` OtherActor))
  (bind _returnvalue (`RPGCharacter.IsDead` _asrpgcharacter))
  (if (not _returnvalue)
    (`self.SetActorHiddenInGame` _asrpgcharacter false)))

(fn `UserConstructionScript`)